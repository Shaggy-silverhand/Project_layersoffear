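; Base interactable item actor that can open an inspection view of its mesh, name and description.
; Construction script applies the configurable sphere radius, mesh and world scale.
; On Interact, inspectable items spawn a BP_InspectItem at a far-off location and pass it the inspection rotation, scale, item data and interacting character.
; Non-inspectable items only print a placeholder message; BeginPlay caches the first-person player character.
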(event EventBeginPlay
  (bind _asbp_first_person_character (Utilities|Casting|CastToBP_FirstPersonCharacter (Game|GetPlayerCharacter 0)))
  (Variables|Public|SetBP%20Player%20Ref _asbp_first_person_character))

(event EventInteract
  (params (Character :type BP%20First%20Person%20Character%20Object%20Reference))
  (if (Variables|Public|GetInspect?)
    (bind _returnvalue (Game|SpawnActorfromClass "/Game/Inspect/BP_InspectItem.BP_InspectItem_C" (Math|Transform|MakeTransform "1000000000.000000,0.000000,0.000000") "Undefined" "MultiplyWithRoot" 0 0))
    (Default|SetInspectRotation _returnvalue (Variables|Public|GetItem%20Inspection%20Rotation))
    (Default|SetInspectScale _returnvalue (Variables|Public|GetItem%20Inspection%20Scale%20))
    (Class|BPIInteract|Inspect(Message) _returnvalue Character (Variables|/Script/Engine.StaticMeshComponent|GetStaticMesh (Variables|Components|GetStaticMesh)) (Variables|Public|GetItem%20Name) (Variables|Public|GetItem%20Description))
    (else
      (Development|PrintString "Hello"))))

(fn ConstructionScript
  (bind _staticmesh (Variables|Components|GetStaticMesh))
  (Utilities|FlowControl|Sequence
    (:then_0
      (Components|Sphere|SetSphereRadius (Variables|Default|GetSphere) (Variables|Default|GetIn%20Sphere%20Radius) true))
    (:then_1
      (Components|StaticMesh|SetStaticMesh (Variables|Components|GetStaticMesh) (Variables|Public|GetItem%20Mesh))
      (Transformation|SetWorldTransform _staticmesh (Math|Transform|MakeTransform (Transformation|GetWorldLocation _staticmesh) (Transformation|GetWorldRotation _staticmesh) (Variables|Public|GetItem%20Scale)) false false))))